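; BP_SS is an actor with a cube, a spring arm and a rotating movement component, configured entirely at construction.
; Its construction script sets the cube's relative transform from initial location, rotation and scale variables, the arm length from Radius, and the movement's rotation rate from RotationRate.
; The event graph holds only disabled placeholder events, leaving runtime motion to the rotating movement component.
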(event EventBeginPlay)

(event Collision|EventActorBeginOverlap
  (params (OtherActor :type Actor%20Object%20Reference)))

(event EventTick
  (params (DeltaSeconds :type Float%20%28single-precision%29)))

(fn ConstructionScript
  (Transformation|SetRelativeTransform (Variables|Default|GetCube) (Math|Transform|MakeTransform (Variables|Cube|GetInitial%20Location) (Variables|Cube|GetInitial%20Rotation) (Variables|Cube|GetScale)) false false)
  (Variables|/Script/Engine.SpringArmComponent|SetTargetArmLength (Variables|Default|GetSpringArm) (Variables|Spinning|GetRadius))
  (Variables|/Script/Engine.RotatingMovementComponent|SetRotationRate (Variables|Default|GetRotatingMovement) (Variables|Spinning|GetRotation%20Rate)))